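; BP_Enemy is an enemy pawn that walks to a fixed offset after spawning and builds awareness of the VR player.
; On BeginPlay it caches the player camera, waits briefly, moves via AI, then tells its AnimBP to attack on arrival.
; Each Tick traces from its eyes to the camera; when unobstructed and the camera is on the positive side of the mesh's right vector, Awareness accumulates over time and is printed.
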(event `self.ReceiveBeginPlay`
  (bind _asbp_vrcharacter (cast `/Game/Blueprints/Player/BP_VRCharacter` (`GameplayStatics.GetPlayerCharacter` 0)))
  (set `self.PlayerCamera` (`/Game/Blueprints/Player/BP_VRCharacter.Camera` _asbp_vrcharacter))
  (`KismetSystemLibrary.Delay` 2.0)
  (`|AIMoveTo` self (+ (`self.K2_GetActorLocation`) (0.0 700.0 0.0)) null
    (:`OnSuccess`
      (`/Game/Blueprints/Enemy/ABP_Enemy.StartAttack` (`self.animBP`)))))

(event `self.ReceiveTick`
  (params (DeltaSeconds :type "Float (single-precision)"))
  (bind _returnvalue (`SceneComponent.K2_GetComponentLocation` (`self.Eyes`)))
  (bind _returnvalue_2 (`SceneComponent.GetRightVector` (`self.Mesh`)))
  (bind _returnvalue_3 (`SceneComponent.K2_GetComponentLocation` (`self.PlayerCamera`)))
  (bind (_outhit _returnvalue_4) (`KismetSystemLibrary.LineTraceSingle` _returnvalue _returnvalue_3 "TraceTypeQuery1"))
  (if _returnvalue_4
    _
    (elif (> (`KismetMathLibrary.VSize` (+ (`KismetMathLibrary.ProjectVectorOnToVector` (`KismetMathLibrary.Normal` (- _returnvalue_3 _returnvalue)) _returnvalue_2) _returnvalue_2)) 1.0)
      (bind _output_get (set `self.awareness` (+ (`self.awareness`) DeltaSeconds)))
      (`KismetSystemLibrary.PrintString` (`KismetStringLibrary.Conv_DoubleToString` _output_get)))))

(fn `UserConstructionScript`
  (`parent.UserConstructionScript`))